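; Clouds actor that scatters cloud meshes in a spherical shell around its origin and slowly spins them.
; The construction script adds HowManyClouds static mesh components, each randomly rotated, then pushed along local Z by MinimumAltitude plus a random Modifier-scaled amount.
; Tick yaws the root by a scaled CloudsSpeed, orbiting all clouds together at a frame-rate-dependent speed.
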(event EventBeginPlay)

(event EventActorBeginOverlap
  (params (OtherActor :type Actor%20Object%20Reference)))

(event EventTick
  (params (DeltaSeconds :type Float%20%28single-precision%29))
  (Transformation|AddRelativeRotation (Variables|Default|GetDefaultSceneRoot) (Math|Rotator|MakeRotator 0.0 0.0 (* (Variables|Default|GetcloudsSpeed) 0.001)) false false))

(fn ConstructionScript
  (for _index (range 1 (Variables|Default|GethowManyClouds))
    (bind _returnvalue (AddComponent|AddStaticMeshComponent false (Math|Transform|MakeTransform "0, 0, 0" (Math|Rotator|MakeRotator (* (Math|Random|RandomFloat) 3.6e+02) (* (Math|Random|RandomFloat) 3.6e+02) (* (Math|Random|RandomFloat) 3.6e+02)))))
    (Transformation|AddLocalOffset _returnvalue (Math|Vector|MakeVector 0.0 0.0 (+ (* (Math|Random|RandomFloat) (Variables|Default|Getmodifier)) (Variables|Default|GetminimumAltitude))) false false)))