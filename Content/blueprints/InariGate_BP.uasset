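; Torii-style Inari gate actor that switches the time of day when the FireflyPawn passes through it, and aligns itself to the gravity direction on BeginPlay.
; On overlap it plays a portal sound, then randomly picks one of the two other DayTime states among day, night and sunset.
; It broadcasts the new state by calling the matching message on every actor implementing the IDayTimeAffected interface.
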(event EventBeginPlay
  (Class|GravityManager|RotateActorAlongGravityDirection self))

(event EventActorBeginOverlap
  (params (OtherActor :type Actor%20Object%20Reference))
  (Utilities|Casting|CastToFireflyPawn OtherActor)
  (Audio|PlaySound2D "/Game/sound/Portail_Jour_-_Nuit_01.Portail_Jour_-_Nuit_01")
  (Utilities|FlowControl|Sequence
    (:then_0
      (CallFunction|SetRandomDayTime))
    (:then_1
      (CallFunction|NotifyDayTime))))

(fn ConstructionScript)

(fn NotifyDayTime
  (bind _outactors (Actor|GetAllActorswithInterface "/Game/blueprints/IDayTimeAffected.IDayTimeAffected_C"))
  (for _array_element _outactors
    (switch int (Variables|Default|GetdayTime)
      (:0
        (Class|IDayTimeAffected|SetDay(Message) _array_element))
      (:1
        (Class|IDayTimeAffected|SetNight(Message) _array_element))
      (:2
        (Class|IDayTimeAffected|SetSunset(Message) _array_element)))))

(fn SetRandomDayTime
  (bind _output_get (LocalVariables|Setrand (Math|Random|RandomInteger 2)))
  (if (< _output_get (Variables|Default|GetdayTime))
    (Variables|Default|SetdayTime _output_get)
    (else
      (Variables|Default|SetdayTime (+ _output_get 1)))))