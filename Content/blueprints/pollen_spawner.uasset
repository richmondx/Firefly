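; Pollen spawner actor that releases a burst of pollen actors at its own transform when a FireflyPawn_BP overlaps it.
; On overlap it reads the pawn's DeltaPollenSpeed and runs a fixed-count spawn loop.
; Each iteration rolls a random integer against that value, so a higher value favors Pollen_BP2 over Pollen_BP.
; A leftover text print is unconnected and never runs.
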(event EventActorBeginOverlap
  (params (OtherActor :type Actor%20Object%20Reference))
  (bind _self self)
  (bind _returnvalue (Transformation|GetActorTransform _self))
  (bind _asfirefly_pawn_bp (Utilities|Casting|CastToFireflyPawn_BP OtherActor))
  (Variables|Default|SetDeltaPollen (Variables|/Game/blueprints/FireflyPawn_BP.FireflyPawn_BP_C|GetdeltaPollenSpeed _asfirefly_pawn_bp))
  (for _index (range 0 10)
    (if (< (Math|Random|RandomIntegerinRange 0 10) (Variables|Default|GetDeltaPollen))
      (Game|SpawnActorfromClass "/Game/blueprints/pollen_BP2.pollen_BP2_C" _returnvalue "Undefined" 0 0)
      (else
        (Game|SpawnActorfromClass "/Game/blueprints/pollen_BP.pollen_BP_C" _returnvalue "Undefined" 0 0)))))

(fn ConstructionScript)