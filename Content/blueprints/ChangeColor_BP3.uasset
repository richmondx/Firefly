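; Actor Blueprint for a tree that changes color when something overlaps its box, then changes again after a timed hold.
; The construction script makes a dynamic material instance on Tree3, whose "vert" vector parameter is driven by two color timelines.
; Overlap plays the first timeline and sets Isinflower, which blocks retriggering.
; Tick uses a one-second Delay to count up to TimeTotal, then clears the flag and plays the second timeline.
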(event OnComponentBeginOverlap(Box)
  (params (OtherActor :type Actor%20Object%20Reference) (OtherComp :type Primitive%20Component%20Object%20Reference) (OtherBodyIndex :type Integer) (bFromSweep :type Boolean) (SweepResult :type Hit%20Result%20Structure%20%28by%20ref%29))
  (if (not (Variables|Default|Getisinflower))
    (Variables|Default|Setisinflower true)
    (bind _color (Timeline|Timeline_0 PlayFromStart)
      (:Update
        (Rendering|Material|SetVectorParameterValue (Variables|Default|GetDynamic%20Material) "vert" (Utilities|Struct|MakeLinearColor (.X (Math|Vector|BreakVector _color)) (.Y (Math|Vector|BreakVector _color)) (.Z (Math|Vector|BreakVector _color)) 0.0) :!class /Script/Engine.MaterialInstanceDynamic)))))

(event EventBeginPlay)

(event Collision|EventActorBeginOverlap
  (params (OtherActor :type Actor%20Object%20Reference)))

(event EventTick
  (params (DeltaSeconds :type Float%20%28single-precision%29))
  (if (Variables|Default|Getisinflower)
    (Utilities|FlowControl|Delay 1.0)
    (if (Variables|Default|Getisinflower)
      (if (== (Variables|Default|GetTime%20counter) (Variables|Default|GetTime%20total))
        (Variables|Default|SetTime%20counter 0)
        (Variables|Default|Setisinflower false)
        (bind _color (Timeline|Timeline_1 PlayFromStart)
          (:Update
            (Rendering|Material|SetVectorParameterValue (Variables|Default|GetDynamic%20Material) "vert" (Utilities|Struct|MakeLinearColor (.X (Math|Vector|BreakVector _color)) (.Y (Math|Vector|BreakVector _color)) (.Z (Math|Vector|BreakVector _color)) 0.0) :!class /Script/Engine.MaterialInstanceDynamic)))
        (else
          (Variables|Default|SetTime%20counter (+ (Variables|Default|GetTime%20counter) 1)))))))

(fn ConstructionScript
  (bind _returnvalue (Rendering|Material|CreateDynamicMaterialInstance (Variables|Default|Gettree3) 0 0 :!class /Script/Engine.PrimitiveComponent))
  (Variables|Default|SetDynamic%20Material _returnvalue))