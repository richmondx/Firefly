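; CactusTrigger is a collectible trigger actor that completes an objective once all instances are picked up.
; When a Pawn overlaps it, it destroys itself and plays a 2D pickup sound, with a redundant second destroy call.
; It then counts the remaining CactusTrigger actors.
; At zero, it teleports the player pawn 500 units up in local space and calls SetSucceded on StateHandler.
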(event Collision|EventActorBeginOverlap
  (params (OtherActor :type Actor%20Object%20Reference))
  (Utilities|Casting|CastToPawn OtherActor)
  (Actor|DestroyActor)
  (Audio|SpawnSound2D "/Game/models/meshs_desert/pickupSound.pickupSound")
  (Actor|DestroyActor)
  (bind _outactors (Actor|GetAllActorsOfClass "cactusTrigger_C"))
  (Math|Integer|CompareInt (Utilities|Array|Length _outactors) 0
    (:==
      _)
    (:<
      _))
  (Transformation|AddActorLocalOffset (Game|Player|GetPlayerPawn 0) "0, 0,500.000000" false true)
  (Default|SetSucceded (Utilities|ResolveSoftReference (Variables|Default|GetstateHandler))))

(event EventBeginPlay)

(event EventActorBeginOverlap
  (params (OtherActor :type Actor%20Object%20Reference)))

(event EventTick
  (params (DeltaSeconds :type Float%20%28single-precision%29)))

(fn ConstructionScript)