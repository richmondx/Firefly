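; Portal actor that teleports the player to a randomly chosen other portal in the level, with its material showing the destination's Location type.
; On BeginPlay it gathers the other portals and picks a destination, re-rolling after each teleport or when the player exits ActivationVolume.
; Entering TeleportVolume moves the player to the destination's EndTeleportVolume.
; The receiving portal disables CanTeleport until the player leaves that volume, preventing an immediate bounce back.
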(event OnComponentEndOverlap(EndTeleportVolume)
  (params (OtherActor :type Actor%20Object%20Reference) (OtherComp :type Primitive%20Component%20Object%20Reference) (OtherBodyIndex :type Integer))
  (if (== OtherActor (Game|Player|GetPlayerPawn 0))
    (Variables|Default|SetCanTeleport true)))

(event OnComponentBeginOverlap(TeleportVolume)
  (params (OtherActor :type Actor%20Object%20Reference) (OtherComp :type Primitive%20Component%20Object%20Reference) (OtherBodyIndex :type Integer) (bFromSweep :type Boolean) (SweepResult :type Hit%20Result%20Structure%20%28by%20ref%29))
  (Development|PrintString "Pouf !")
  (if (and (== OtherActor (Game|Player|GetPlayerPawn 0)) (Variables|Default|GetCanTeleport))
    (Development|PrintString "Prout !")
    (CallFunction|Teleport (Variables|Default|GetDestination) OtherActor)
    (CallFunction|SetRandomDestination)))

(event OnComponentEndOverlap(ActivationVolume)
  (params (OtherActor :type Actor%20Object%20Reference) (OtherComp :type Primitive%20Component%20Object%20Reference) (OtherBodyIndex :type Integer))
  (if (== OtherActor (Game|Player|GetPlayerPawn 0))
    (CallFunction|SetRandomDestination)))

(event EventBeginPlay
  (Utilities|FlowControl|Sequence
    (:then_0
      (bind _outactors (Actor|GetAllActorsOfClass "Portal_BP_C"))
      (for _array_element _outactors
        (if (!= _array_element self)
          (Utilities|Array|Add (Variables|Default|GetPortals) _array_element))))
    (:then_1
      (CallFunction|SetRandomDestination))))

(fn ConstructionScript)

(fn SetRandomDestination
  (bind _portals (Variables|Default|GetPortals))
  (bind _staticmesh (Variables|Default|GetStaticMesh))
  (bind _output_get (Variables|Default|SetDestination (Utilities|Array|Get(acopy) _portals (Math|Random|RandomIntegerinRange 0 (- (Utilities|Array|Length _portals) 1)))))
  (switch Utilities|FlowControl|Switch|SwitchonPortal_ENUM (Variables|Portal_BP_C|GetLocation _output_get)
    (:NewEnumerator0
      (Rendering|Material|SetMaterial _staticmesh 2 "/Game/materials/Portal_material_Country.Portal_material_Country"))
    (:NewEnumerator1
      (Rendering|Material|SetMaterial _staticmesh 2 "/Game/materials/Portal_material_Moutain.Portal_material_Moutain"))
    (:NewEnumerator2
      (Rendering|Material|SetMaterial _staticmesh 2 "/Game/materials/Portal_material_Desert.Portal_material_Desert"))
    (:NewEnumerator3
      (Rendering|Material|SetMaterial _staticmesh 2 "/Game/materials/Portal_material_Town.Portal_material_Town"))))

(fn Teleport
  (params (Pawn :type Actor%20Object%20Reference))
  (Variables|Default|SetCanTeleport false)
  (Transformation|SetActorLocation Pawn (Transformation|GetWorldLocation (Variables|Default|GetEndTeleportVolume)) false false))