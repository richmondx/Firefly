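; Grass scatter actor that procedurally places static mesh components, presumably grass, around its origin.
; The construction script adds HowManyGrass meshes, each offset by the X and Y of random unit vectors scaled by Modifer, on a flat Z of zero.
; All instances keep zero rotation and unit scale, as the random angle calculation is left unconnected.
; The event graph has no active logic.
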(event EventBeginPlay)

(event EventActorBeginOverlap
  (params (OtherActor :type Actor%20Object%20Reference)))

(event EventTick
  (params (DeltaSeconds :type Float%20%28single-precision%29)))

(fn ConstructionScript
  (bind _returnvalue (Math|Random|RandomUnitVector))
  (bind _modifer (Variables|Default|Getmodifer))
  (bind _returnvalue_2 (* _returnvalue _modifer))
  (bind (_x _y) (Math|Vector|BreakVector _returnvalue_2))
  (for _index (range 1 (Variables|Default|GethowManyGrass))
    (AddComponent|AddStaticMeshComponent false (Math|Transform|MakeTransform (Math|Vector|MakeVector _x _y 0.0) (Math|Rotator|MakeRotator 0.0 0.0 0.0)))))