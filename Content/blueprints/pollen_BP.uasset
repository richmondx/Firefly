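; Pollen pickup actor that gives the player's firefly pawn a speed boost.
; On BeginPlay, a timeline drifts it along a random, upward-biased local offset as a spawn motion.
; When a firefly pawn overlaps it, it increments the pawn's pollen speed counter, calls Boost, plays a 2D acceleration sound and destroys itself.
; A second timeline for light intensity and mesh position is unconnected and never runs.
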(event Collision|EventActorBeginOverlap
  (params (OtherActor :type Actor%20Object%20Reference))
  (bind _asfirefly_pawn_bp (Utilities|Casting|CastToFireflyPawn_BP OtherActor))
  (Math|Integer|IncrementInt (Variables|/Game/blueprints/FireflyPawn_BP.FireflyPawn_BP_C|GetdeltaPollenSpeed _asfirefly_pawn_bp)
    (:%20%20
      (bind _asfirefly_pawn (Utilities|Casting|CastToFireflyPawn OtherActor))
      (Class|FireflyPawn|Boost _asfirefly_pawn)
      (Audio|SpawnSound2D "/Game/sound/Pollen_-_Accélérer_01.Pollen_-_Accélérer_01")
      (Actor|DestroyActor self))))

(event EventBeginPlay
  (Variables|Default|SetrandX (Math|Random|RandomFloatinRange -4.0 4.0))
  (Variables|Default|SetrandY (Math|Random|RandomFloatinRange -4.0 4.0))
  (Variables|Default|SetrandZ (Math|Random|RandomFloatinRange 2.0 6.0))
  (bind _movement (Timeline|SpawnMovement Play)
    (:Update
      (Variables|Default|Setmovement (* _movement 1.0))
      (Transformation|AddLocalOffset (Variables|Default|GetDefaultSceneRoot1) (Math|Vector|MakeVector (* (Variables|Default|Getmovement) (Variables|Default|GetrandX)) (* (Variables|Default|Getmovement) (Variables|Default|GetrandY)) (* (Variables|Default|Getmovement) (Variables|Default|GetrandZ))) false false))))

(fn ConstructionScript)