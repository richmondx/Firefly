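; Portal actor that teleports an overlapping FireflyPawn to a randomly picked other portal in the level.
; On BeginPlay it stores every other Portal_BP; on overlap it moves the pawn to a portal's LocationToTeleport.
; An IsTeleporting flag, cleared on end overlap, blocks re-triggering, but the flagged portal and the destination are rolled separately, so they can differ.
; A collapse sound node is present but never runs.
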(event EventBeginPlay
  (bind _outactors (Actor|GetAllActorsOfClass "Portal_BP_C"))
  (for _array_element _outactors
    (if (!= _array_element self)
      (Utilities|Array|Add (Variables|Default|GetOtherPortals) _array_element))))

(event EventActorBeginOverlap
  (params (OtherActor :type Actor%20Object%20Reference))
  (bind _otherportals (Variables|Default|GetOtherPortals))
  (bind _returnvalue (Utilities|Array|Length _otherportals))
  (bind _returnvalue_2 (- _returnvalue 1))
  (bind _returnvalue_3 (Math|Random|RandomIntegerinRange 0 _returnvalue_2))
  (bind _item (Utilities|Array|Get(acopy) _otherportals _returnvalue_3))
  (if (not (Variables|Default|GetIsTeleporting))
    (bind _asfirefly_pawn (Utilities|Casting|CastToFireflyPawn OtherActor))
    (Variables|Portal_BP_C|SetIsTeleporting _item true)
    (Transformation|SetActorLocation _asfirefly_pawn (Transformation|GetWorldLocation (Variables|Portal_BP_C|GetLocationToTeleport _item)) false true)))

(event Collision|EventActorEndOverlap
  (params (OtherActor :type Actor%20Object%20Reference))
  (Utilities|Casting|CastToFireflyPawn OtherActor)
  (Variables|Default|SetIsTeleporting false))

(fn ConstructionScript)