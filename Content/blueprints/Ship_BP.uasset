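; Moving ship that follows a trajectory over accumulated time, aligns to gravity each tick and carries the FireflyPawn as a passenger.
; Two trigger boxes share a reference count, so the pawn attaches to the ship on the first overlap, keeping its world position.
; It detaches only when the count drops back to zero, letting it cross between the boxes without falling off.
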(event OnComponentBeginOverlap(Box)
  (params (OtherActor :type Actor%20Object%20Reference) (OtherComp :type Primitive%20Component%20Object%20Reference) (OtherBodyIndex :type Integer) (bFromSweep :type Boolean) (SweepResult :type Hit%20Result%20Structure%20%28by%20ref%29))
  (bind _asfirefly_pawn (Utilities|Casting|CastToFireflyPawn OtherActor))
  (Variables|Default|SetPassenger _asfirefly_pawn)
  (bind _result (Math|Integer|IncrementInt (Variables|Default|GetNbRef))
    (:%20%20
      (if (== _result 1)
        (Class|Actor|AttachRootComponenttoActor (Variables|Default|GetPassenger) self "None" "KeepWorldPosition" false)))))

(event OnComponentBeginOverlap(Box1)
  (params (OtherActor :type Actor%20Object%20Reference) (OtherComp :type Primitive%20Component%20Object%20Reference) (OtherBodyIndex :type Integer) (bFromSweep :type Boolean) (SweepResult :type Hit%20Result%20Structure%20%28by%20ref%29))
  (bind _asfirefly_pawn (Utilities|Casting|CastToFireflyPawn OtherActor))
  (Variables|Default|SetPassenger _asfirefly_pawn)
  (bind _result (Math|Integer|IncrementInt (Variables|Default|GetNbRef))
    (:%20%20
      (if (== _result 1)
        (Class|Actor|AttachRootComponenttoActor (Variables|Default|GetPassenger) self "None" "KeepWorldPosition" false)))))

(event OnComponentEndOverlap(Box)
  (params (OtherActor :type Actor%20Object%20Reference) (OtherComp :type Primitive%20Component%20Object%20Reference) (OtherBodyIndex :type Integer))
  (bind _nbref (Variables|Default|GetNbRef))
  (Utilities|Casting|CastToFireflyPawn OtherActor)
  (if (> _nbref 0)
    (bind _result (Math|Integer|DecrementInt _nbref)
      (:%20%20
        (if (== _result 0)
          (Class|Actor|DetachRootComponentfromParent (Variables|Default|GetPassenger) true))))))

(event OnComponentEndOverlap(Box1)
  (params (OtherActor :type Actor%20Object%20Reference) (OtherComp :type Primitive%20Component%20Object%20Reference) (OtherBodyIndex :type Integer))
  (bind _nbref (Variables|Default|GetNbRef))
  (Utilities|Casting|CastToFireflyPawn OtherActor)
  (if (> _nbref 0)
    (bind _result (Math|Integer|DecrementInt _nbref)
      (:%20%20
        (if (== _result 0)
          (Class|Actor|DetachRootComponentfromParent (Variables|Default|GetPassenger) true))))))

(event EventTick
  (params (DeltaSeconds :type Float%20%28single-precision%29))
  (bind _self self)
  (bind _output_get (Variables|Default|SetElapsedTime (+ DeltaSeconds (Variables|Default|GetElapsedTime))))
  (Class|Trajectory|Follow (Variables|Trajectory|GetTrajectory) _self _output_get)
  (Class|GravityManager|RotateActorAlongGravityDirection _self))

(fn ConstructionScript)