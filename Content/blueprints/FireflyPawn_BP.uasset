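; FireflyPawn_BP is a firefly pawn that toggles streetlamp (Lampadaire_BP) lights by looking at them.
; Each tick, it calls OrientateCameraAlongHMD when a headset is enabled, then runs a short Visibility line trace along the camera's forward vector.
; On a hit that passes a LastActorAimed check against Lampadaire_BP_C, it casts to Lampadaire_BP, calls ToggleLight and stores that actor as LastActorAimed.
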(event EventTick
  (params (DeltaSeconds :type Float%20%28single-precision%29))
  (bind _m_camera (Variables|Default|Getm_camera))
  (bind _returnvalue (Transformation|GetWorldLocation _m_camera))
  (if (Class|HeadMountedDisplayFunctionLibrary|IsHeadMountedDisplayEnabled)
    (Class|FireflyPawn|OrientateCameraAlongHMD))
  ;[1 1 1] Aim Interactions
  (bind (_outhit _returnvalue_2) (Collision|LineTraceByChannel 0 _returnvalue (+ _returnvalue (* (Math|Vector|GetForwardVector _m_camera) 500)) "TraceTypeQuery1" false 0 "None"))
  (if _returnvalue_2
    (if (!= (Variables|Default|GetlastActorAimed) "/Game/blueprints/Lampadaire_BP.Lampadaire_BP_C")
      (bind _aslampadaire_bp (Utilities|Casting|CastToLampadaire_BP (.HitActor (Collision|BreakHitResult _outhit))))
      (Default|ToggleLight _aslampadaire_bp)
      (Variables|Default|SetlastActorAimed (.HitActor (Collision|BreakHitResult _outhit))))))

(fn ConstructionScript)