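; Desert fire trigger actor that starts a timed round of TriggerCactus_Blueprint actors in the level.
; Any actor overlap resets TimeLeft to TimeCountDown and spawns a cactus trigger at every TargetPoint.
; Tick counts TimeLeft down through a one-second Delay, which throttles the per-frame calls.
; Once TimeLeft drops below zero, Tick destroys every TriggerCactus_Blueprint in the level.
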(event EventTick
  (params (DeltaSeconds :type Float%20%28single-precision%29))
  (Math|Integer|CompareInt (Variables|Default|GettimeLeft) 0
    (:>
      (Utilities|FlowControl|Delay 1.0 :!label _label)
      (Variables|Default|SettimeLeft (- (Variables|Default|GettimeLeft) 1)))
    (:==
      (goto _label))
    (:<
      (bind _outactors (Actor|GetAllActorsOfClass "/Game/blueprints/triggerCactus-_Blueprint.triggerCactus-_Blueprint_C"))
      (for _array_element _outactors
        (Actor|DestroyActor _array_element)))))

(event EventBeginPlay)

(event EventActorBeginOverlap
  (params (OtherActor :type Actor%20Object%20Reference)))

(event EventTick
  (params (DeltaSeconds :type Float%20%28single-precision%29)))

(event Collision|EventActorBeginOverlap
  (params (OtherActor :type Actor%20Object%20Reference))
  (Variables|Default|SettimeLeft (Variables|Default|GettimeCountDown))
  (bind _outactors (Actor|GetAllActorsOfClass "/Script/Engine.TargetPoint"))
  (for _array_element _outactors
    (Game|SpawnActorfromClass "/Game/blueprints/triggerCactus-_Blueprint.triggerCactus-_Blueprint_C" (Transformation|GetActorTransform _array_element) "AlwaysSpawn" 0 0)))

(fn ConstructionScript)