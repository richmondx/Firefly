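; Street lamp Blueprint that switches its lamp between on and off looks by swapping materials.
; The ToggleLight event alternates between the on and off lamp materials and applies the result to one material slot of the Lampadaire component.
; A real-time cooldown of one second between toggles prevents the lamp from flipping every frame.
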(event Custom|ToggleLight
  ;[1 1 1] Prevent toggling every frame
  (if (> (- (Utilities|Time|GetRealTimeSeconds) (Variables|Default|GetlastToggleTime)) 1.0)
    (if (== (Variables|Default|GetmaterialLight) "/Game/models/meshs_ville/lampadaireLampeOff.lampadaireLampeOff")
      (Variables|Default|SetmaterialLight "/Game/models/meshs_ville/lampadaireLampeOn.lampadaireLampeOn")
      (else
        (Variables|Default|SetmaterialLight "/Game/models/meshs_ville/lampadaireLampeOff.lampadaireLampeOff")))
    (Rendering|Material|SetMaterial (Variables|Default|Getlampadaire) 1 (Variables|Default|GetmaterialLight))
    (Variables|Default|SetlastToggleTime (Utilities|Time|GetRealTimeSeconds))))

(fn ConstructionScript)