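; Short-lived pollen actor that brakes the firefly pawn on contact and plays a slowdown sound.
; On BeginPlay, timelines drift it along a random, upward-biased offset and animate its scale, destroying it when scaling finishes.
; Actor overlap also decrements the pawn's DeltaPollenSpeed and destroys the pollen.
; A separate Box overlap handler instead hides and re-shows the mesh after RespawnTime, while two light/position timelines are never triggered.
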(event OnComponentBeginOverlap(Box)
  (params (OtherActor :type Actor%20Object%20Reference) (OtherComp :type Primitive%20Component%20Object%20Reference) (OtherBodyIndex :type Integer) (bFromSweep :type Boolean) (SweepResult :type Hit%20Result%20Structure%20%28by%20ref%29))
  (bind _pollen (Variables|Default|Getpollen))
  (bind _asfirefly_pawn (Utilities|Casting|CastToFireflyPawn OtherActor))
  (Class|FireflyPawn|Brake _asfirefly_pawn)
  (Rendering|SetVisibility _pollen false false)
  (Audio|SpawnSound2D "/Game/sound/Pollen_-_Ralentir_01.Pollen_-_Ralentir_01")
  (Utilities|FlowControl|Delay (Variables|Default|GetrespawnTime))
  (Rendering|SetVisibility _pollen true false))

(event Collision|EventActorBeginOverlap
  (params (OtherActor :type Actor%20Object%20Reference))
  (bind _asfirefly_pawn_bp (Utilities|Casting|CastToFireflyPawn_BP OtherActor))
  (Math|Integer|DecrementInt (Variables|/Game/blueprints/FireflyPawn_BP.FireflyPawn_BP_C|GetdeltaPollenSpeed _asfirefly_pawn_bp)
    (:%20%20
      (bind _asfirefly_pawn (Utilities|Casting|CastToFireflyPawn OtherActor))
      (Class|FireflyPawn|Brake _asfirefly_pawn)
      (Audio|SpawnSound2D "/Game/sound/Pollen_-_Ralentir_01.Pollen_-_Ralentir_01")
      (Actor|DestroyActor self))))

(event EventBeginPlay
  (bind _self self)
  (Variables|Default|SetrandX (Math|Random|RandomFloatinRange -4.0 4.0))
  (Variables|Default|SetrandY (Math|Random|RandomFloatinRange -4.0 4.0))
  (Variables|Default|SetrandZ (Math|Random|RandomFloatinRange 2.0 6.0))
  (Utilities|FlowControl|Sequence
    (:then_0
      (bind _movement (Timeline|Timeline_2 Play)
        (:Update
          (Variables|Default|Setmovement (* _movement 1.0))
          (Transformation|AddLocalOffset (Variables|Default|GetDefaultSceneRoot1) (* (Math|Vector|MakeVector (* (Variables|Default|Getmovement) (Variables|Default|GetrandX)) (* (Variables|Default|Getmovement) (Variables|Default|GetrandY)) (* (Variables|Default|Getmovement) (Variables|Default|GetrandZ))) 2.0) false false))))
    (:then_1
      (bind _scaleparameter (Timeline|Timeline_3 Play)
        (:Update
          (Transformation|SetActorScale3D _self (Math|Conversions|ToVector(Float) _scaleparameter)))
        (:Finished
          (Actor|DestroyActor _self))))))

(fn ConstructionScript)