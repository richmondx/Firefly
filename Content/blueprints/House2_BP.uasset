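; House Blueprint with a ToggleLight event that switches its lamp material and four point lights on or off.
; A one-second cooldown, restarted only on material swaps, gates the event, and the current material selects the on or off branch.
; Each branch uses a looping MultiGate, so each call performs only one light change or material swap.
; PointLight3's on step sets indirect lighting intensity rather than intensity.
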(event Custom|ToggleLight
  ;[1 1 1] Prevent toggling every frame
  (if (> (- (Utilities|Time|GetRealTimeSeconds) (Variables|Default|GetlastToggleTime)) 1.0)
    (if (== (Variables|Default|GetmaterialLight) "/Game/models/meshs_ville/lampadaireLampeOff.lampadaireLampeOff")
      (Utilities|FlowControl|MultiGate false true -1
        (:Out%200
          (Class|LightComponent|SetIndirectLightingIntensity (Variables|Default|GetPointLight3) 2.5e+05))
        (:Out%201
          (Rendering|Components|Light|SetIntensity (Variables|Default|GetPointLight2) 2.5e+05))
        (:Out%202
          (Rendering|Components|Light|SetIntensity (Variables|Default|GetPointLight1) 2.5e+05))
        (:Out%203
          (Rendering|Components|Light|SetIntensity (Variables|Default|GetPointLight) 2.5e+05))
        (:Out%204
          (Variables|Default|SetmaterialLight "/Game/models/meshs_ville/lampadaireLampeOn.lampadaireLampeOn")
          (Rendering|Material|SetMaterial (Variables|Default|GetHouse2) 5 (Variables|Default|GetmaterialLight) :!label _label)
          (Variables|Default|SetlastToggleTime (Utilities|Time|GetRealTimeSeconds))))
      (else
        (Utilities|FlowControl|MultiGate false true -1
          (:Out%200
            (Variables|Default|SetmaterialLight "/Game/models/meshs_ville/lampadaireLampeOff.lampadaireLampeOff")
            (goto _label))
          (:Out%201
            (Rendering|Components|Light|SetIntensity (Variables|Default|GetPointLight) 0.0))
          (:Out%202
            (Rendering|Components|Light|SetIntensity (Variables|Default|GetPointLight1) 0.0))
          (:Out%203
            (Rendering|Components|Light|SetIntensity (Variables|Default|GetPointLight2) 0.0))
          (:Out%204
            (Rendering|Components|Light|SetIntensity (Variables|Default|GetPointLight3) 0.0)))))))

(fn ConstructionScript)