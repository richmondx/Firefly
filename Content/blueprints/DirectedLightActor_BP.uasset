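; DirectedLightActor_BP is a light actor with day and night intensity levels.
; On BeginPlay it stores the player pawn as Target and enables actor tick if that pawn is valid, though the graph holds no Tick logic of its own.
; SetDay and SetNight events switch the MLight component between DayIntensity and NightIntensity.
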(event EventBeginPlay
  (bind _returnvalue (Game|Player|GetPlayerPawn 0))
  (Utilities|IsValid _returnvalue
    (:Is%20Valid
      (Variables|Default|SetTarget _returnvalue)
      (Actor|Tick|SetActorTickEnabled true))))

(event EventSetDay
  (Rendering|Components|Light|SetIntensity (Variables|Default|Getm_light) (Variables|Default|GetDayIntensity)))

(event EventSetNight
  (Rendering|Components|Light|SetIntensity (Variables|Default|Getm_light) (Variables|Default|GetNightIntensity)))

(fn ConstructionScript)