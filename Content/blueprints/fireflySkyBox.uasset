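; Skybox actor that switches the sky between day, night and sunset looks.
; SetDay, SetNight and SetSunset events each store the matching material in SkyboxMaterial, then call SetSkyboxMaterial.
; That function applies the material to element 0 of six face components: Front, Back, Gauche, Droite, Haut and Bas.
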(event EventBeginPlay)

(event EventActorBeginOverlap
  (params (OtherActor :type Actor%20Object%20Reference)))

(event EventTick
  (params (DeltaSeconds :type Float%20%28single-precision%29)))

(event EventSetDay
  (Variables|Default|SetskyboxMaterial "/Game/models/models_world/skybox_material_day.skybox_material_day")
  (CallFunction|SetSkyboxMaterial))

(event EventSetSunset
  (Variables|Default|SetskyboxMaterial "/Game/models/models_world/skybox_material_sunset.skybox_material_sunset")
  (CallFunction|SetSkyboxMaterial))

(event EventSetNight
  (Variables|Default|SetskyboxMaterial "/Game/models/models_world/skybox_material_night.skybox_material_night")
  (CallFunction|SetSkyboxMaterial))

(fn ConstructionScript)

(fn SetSkyboxMaterial
  (Rendering|Material|SetMaterial (Variables|Default|Getfront) 0 (Variables|Default|GetskyboxMaterial))
  (Rendering|Material|SetMaterial (Variables|Default|Getback) 0 (Variables|Default|GetskyboxMaterial))
  (Rendering|Material|SetMaterial (Variables|Default|Getgauche) 0 (Variables|Default|GetskyboxMaterial))
  (Rendering|Material|SetMaterial (Variables|Default|Gethaut) 0 (Variables|Default|GetskyboxMaterial))
  (Rendering|Material|SetMaterial (Variables|Default|Getbas) 0 (Variables|Default|GetskyboxMaterial))
  (Rendering|Material|SetMaterial (Variables|Default|Getdroite) 0 (Variables|Default|GetskyboxMaterial)))